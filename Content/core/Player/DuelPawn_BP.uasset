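; DuelPawn_BP is a player pawn with free-floating movement and look controls.
; Forward and right axis inputs feed FloatingPawnMovement along the Camera's forward and right vectors, so forward movement follows the view direction.
; Turn and LookUp axes drive controller yaw and pitch.
; Fire is a placeholder that only prints start and stop messages, and the construction script is empty.
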(event `InputAxis|MoveForward`
  (params (AxisValue :type "Float (single-precision)"))
  ;[1 1 1] Input
  (`PawnMovementComponent.AddInputVector` (`self.FloatingPawnMovement`) (* (`SceneComponent.GetForwardVector` (`self.Camera`)) AxisValue) false))

(event `InputAxis|MoveRight`
  (params (AxisValue :type "Float (single-precision)"))
  ;[1 1 1] Input
  (`PawnMovementComponent.AddInputVector` (`self.FloatingPawnMovement`) (* (`SceneComponent.GetRightVector` (`self.Camera`)) AxisValue) false))

(event `InputAxis|LookUp`
  (params (AxisValue :type "Float (single-precision)"))
  ;[1 1 1] Input
  (`self.AddControllerPitchInput` AxisValue))

(event `InputAxis|Turn`
  (params (AxisValue :type "Float (single-precision)"))
  ;[1 1 1] Input
  (`self.AddControllerYawInput` AxisValue))

(event `InputAction|Fire`
  (params (Key :type "Key Structure"))
  ;[1 1 1] Input
  (:`Pressed`
    (`KismetSystemLibrary.PrintString` "Fire start"))
  (:`Released`
    (`KismetSystemLibrary.PrintString` "Fire stop")))

(fn `UserConstructionScript`)